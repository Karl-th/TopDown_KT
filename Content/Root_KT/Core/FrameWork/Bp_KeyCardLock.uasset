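; Keycard-locked door actor that opens when a CorePlayerCharacter holding both keycards enters its trigger.
; The Trigger overlap checks both keycard flags on the player and prints a message if either is missing.
; With both, a DoorOpen timeline lerps between start and end vectors and builds a rotation from the result's Z axis.
; That rotation is applied to the whole actor, leaving the Door variable unused.
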(event OnComponentBeginOverlap(Trigger)
  (params (OverlappedComponent :type Primitive%20Component%20Object%20Reference) (OtherActor :type Actor%20Object%20Reference) (OtherComp :type Primitive%20Component%20Object%20Reference) (OtherBodyIndex :type Integer) (bFromSweep :type Boolean) (SweepResult :type Hit%20Result%20Structure%20%28by%20ref%29))
  (bind _ascore_player_character (Utilities|Casting|CastToCorePlayerCharacter OtherActor))
  (if (and (Variables|/Game/Root_KT/Core/FrameWork/CorePlayerCharacter.CorePlayerCharacter_C|GetKeycard1 _ascore_player_character) (Variables|/Game/Root_KT/Core/FrameWork/CorePlayerCharacter.CorePlayerCharacter_C|GetKeycard2 _ascore_player_character))
    (bind _newtrack_0 (Timeline|DoorOpen Play)
      (:Update
        (Transformation|SetActorRelativeRotation (Math|Rotator|MakeRotfromZ (Math|Vector|Lerp(Vector) (Variables|Default|GetStartPos) (Variables|Default|GetEndPos) _newtrack_0)))))
    (else
      (Development|PrintString "Two keys needed"))))

(fn ConstructionScript)