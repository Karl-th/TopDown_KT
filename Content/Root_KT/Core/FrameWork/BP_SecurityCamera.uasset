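; BP_SecurityCamera is a security camera that detects the player and can be switched off at a switchboard.
; While activated, it flags a CorePlayerCharacter entering Trigger as detected, prints a debug message and turns its spotlight red, reverting on exit.
; A second volume, Trigger2, enables input on overlap so pressing E deactivates the camera and zeroes the light's intensity, with no reactivation.
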(event OnComponentBeginOverlap(Trigger)
  (params (OverlappedComponent :type Primitive%20Component%20Object%20Reference) (OtherActor :type Actor%20Object%20Reference) (OtherComp :type Primitive%20Component%20Object%20Reference) (OtherBodyIndex :type Integer) (bFromSweep :type Boolean) (SweepResult :type Hit%20Result%20Structure%20%28by%20ref%29))
  ;[1 1 1] Camera discovers you when entering trigger
  (Utilities|Casting|CastToCorePlayerCharacter OtherActor)
  (if (Variables|Default|GetActivated)
    (Development|PrintString "Detected")
    (Rendering|Components|Light|SetLightColor (Variables|Default|GetSpotLight) "(R=1.000000,G=0.000000,B=0.007892,A=1.000000)" true)
    (Variables|Default|SetPlayerDetect true)))

(event OnComponentEndOverlap(Trigger)
  (params (OverlappedComponent :type Primitive%20Component%20Object%20Reference) (OtherActor :type Actor%20Object%20Reference) (OtherComp :type Primitive%20Component%20Object%20Reference) (OtherBodyIndex :type Integer))
  ;[1 1 1] Camera discovers you when entering trigger
  (Utilities|Casting|CastToCorePlayerCharacter OtherActor)
  (Rendering|Components|Light|SetLightColor (Variables|Default|GetSpotLight) "(R=1.000000,G=0.964686,B=0.571125,A=1.000000)" true)
  (Variables|Default|SetPlayerDetect false))

(event OnComponentBeginOverlap(Trigger2)
  (params (OverlappedComponent :type Primitive%20Component%20Object%20Reference) (OtherActor :type Actor%20Object%20Reference) (OtherComp :type Primitive%20Component%20Object%20Reference) (OtherBodyIndex :type Integer) (bFromSweep :type Boolean) (SweepResult :type Hit%20Result%20Structure%20%28by%20ref%29))
  ;[1 1 1] Enable input
  (Input|EnableInput (Game|GetPlayerController 0)))

(event OnComponentEndOverlap(Trigger2)
  (params (OverlappedComponent :type Primitive%20Component%20Object%20Reference) (OtherActor :type Actor%20Object%20Reference) (OtherComp :type Primitive%20Component%20Object%20Reference) (OtherBodyIndex :type Integer))
  ;[1 1 1] Enable input
  (Input|DisableInput (Game|GetPlayerController 0)))

(event Input|KeyboardEvents|E
  (params (Key :type Key%20Structure))
  ;[1 1 1] SwitchBoard to deactivate camera
  (:Pressed
    (Variables|Default|SetActivated false)
    (Rendering|Components|Light|SetIntensity (Variables|Default|GetSpotLight) 0.0)))

(fn ConstructionScript)