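; BP_SplinePatrol is a patrol actor that moves along a spline and detects the player.
; Each Tick it advances the sphere along the spline at constant speed, matching position and rotation, and wraps to the start at the end.
; A trigger overlap with CorePlayerCharacter halts the patrol and turns the spotlight red.
; Ending the overlap restores the warm light color and resumes movement.
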(event OnComponentBeginOverlap(Trigger)
  (params (OverlappedComponent :type Primitive%20Component%20Object%20Reference) (OtherActor :type Actor%20Object%20Reference) (OtherComp :type Primitive%20Component%20Object%20Reference) (OtherBodyIndex :type Integer) (bFromSweep :type Boolean) (SweepResult :type Hit%20Result%20Structure%20%28by%20ref%29))
  ;[1 1 1] Identifying Layer
  (Utilities|Casting|CastToCorePlayerCharacter OtherActor)
  (Development|PrintString "Detected")
  (Rendering|Components|Light|SetLightColor (Variables|Default|GetSpotLight) "(R=1.000000,G=0.000000,B=0.007892,A=1.000000)" true)
  (Variables|Default|SetPlayerDetected true))

(event OnComponentEndOverlap(Trigger)
  (params (OverlappedComponent :type Primitive%20Component%20Object%20Reference) (OtherActor :type Actor%20Object%20Reference) (OtherComp :type Primitive%20Component%20Object%20Reference) (OtherBodyIndex :type Integer))
  ;[1 1 1] Identifying Layer
  (Utilities|Casting|CastToCorePlayerCharacter OtherActor)
  (Rendering|Components|Light|SetLightColor (Variables|Default|GetSpotLight) "(R=1.000000,G=0.964686,B=0.571125,A=1.000000)" true)
  (Variables|Default|SetPlayerDetected false))

(event EventTick
  (params (DeltaSeconds :type Float%20%28single-precision%29))
  (bind _spline (Variables|Default|GetSpline))
  (bind _returnvalue (Spline|GetSplineLength _spline))
  ;[1 1 1] Rotating on Spline
  (if (not (Variables|Default|GetPlayerDetected))
    (if (>= (Variables|Default|GetCurrentDistanceAlongSpine) _returnvalue)
      (Variables|Default|SetCurrentDistanceAlongSpine 0.0)
      (else
        (bind _output_get (Variables|Default|SetCurrentDistanceAlongSpine (Math|Interpolation|FInterptoConstant (Variables|Default|GetCurrentDistanceAlongSpine) _returnvalue DeltaSeconds 2e+02)))
        (Transformation|SetRelativeLocationAndRotation (Variables|Default|GetSphere) (Spline|GetLocationatDistanceAlongSpline (Variables|Default|GetSpline) _output_get "Local") (Spline|GetRotationatDistanceAlongSpline (Variables|Default|GetSpline) _output_get "Local") false false)))))

(fn ConstructionScript)